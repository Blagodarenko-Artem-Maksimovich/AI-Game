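; BP_InteractableSkeletalMesh is an interactable actor that displays a configurable skeletal mesh and exposes data that appears to describe how it is held.
; Its construction script applies SkeletalMeshSpawn to the SkeletalMesh component.
; GetInfo returns that mesh along with the left-handle value, offset and hand type for callers.
; The event graph holds only disabled default events, so the actor has no runtime logic of its own.
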(fn `GetInfo`
  (returns (StaticMesh :type "StaticMesh Object Reference") (SkeletalMesh :type "SkeletalMesh Object Reference") (LeftHendl :type Boolean) (Offset :type "Vector Structure") (HeandType :type "/Game/AdvancedLocomotionV4/Data/Enums/ALS_OverlayState Enum"))
  (return null (`self.SkeletalMeshSpawn`) (`self.Left Hendl`) (`self.Offset`) (`self.TypeObj`)))

(fn `UserConstructionScript`
  (`SkinnedMeshComponent.SetSkinnedAssetAndUpdate` (`self.SkeletalMesh`) (`self.SkeletalMeshSpawn`) true))