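; BP_InteractableBase is a base interactable that deals hit damage when moving fast and exposes hand-related info.
; On overlap, if the Capsule's physics speed exceeds a threshold, it sends HitMessage to the other actor with that velocity as impulse, the actor's location and fixed damage.
; The FriendWeapon flag exempts actors whose class is exactly TopDownCharacter.
; GetInfo returns the left-hand value, offset and hand type.
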(event `self.ReceiveActorBeginOverlap`
  (params (OtherActor :type "Actor Object Reference"))
  (bind _returnvalue (`PrimitiveComponent.GetPhysicsLinearVelocity` (`self.Capsule`) "None"))
  (if (> (`KismetMathLibrary.VSize` _returnvalue) 750.0)
    (if (`self.FriendWeapon`)
      (if (not (== (`GameplayStatics.GetObjectClass` OtherActor) "/Game/TopDownBP/Blueprints/TopDownCharacter.TopDownCharacter_C"))
        (message `/Game/TopDownBP/Blueprints/BPI_Hit.Hit` OtherActor _returnvalue (`self.K2_GetActorLocation` OtherActor) "None" 20.0 :!label _label))
      (else
        (goto _label)))))

(fn `GetInfo`
  (returns (StaticMesh :type "StaticMesh Object Reference") (SkeletalMesh :type "SkeletalMesh Object Reference") (LeftHendl :type Boolean) (Offset :type "Vector Structure") (HeandType :type "/Game/AdvancedLocomotionV4/Data/Enums/ALS_OverlayState Enum"))
  (return null null (`self.Left Hendl`) (`self.Offset`) (`self.TypeObj`)))

(fn `UserConstructionScript`)